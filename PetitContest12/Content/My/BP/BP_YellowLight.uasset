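; BP_YellowLight is a light actor that turns the player yellow on overlap and can patrol back and forth.
; BeginPlay caches the ThirdPersonCharacter, and when the player pawn enters the Cube, that character's NowYellow flag is set and its red, green and blue flags are cleared.
; When MoveFlag is on, Tick steps it along Y or X (chosen by RIghtLeftFlag), reversing at MaxValue and LowValue at a frame-rate-dependent speed.
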(event OnComponentBeginOverlap(Cube)
  (params (OverlappedComponent :type Primitive%20Component%20Object%20Reference) (OtherActor :type Actor%20Object%20Reference) (OtherComp :type Primitive%20Component%20Object%20Reference) (OtherBodyIndex :type Integer) (bFromSweep :type Boolean) (SweepResult :type Hit%20Result%20Structure%20%28by%20ref%29))
  (bind _thirdpersoncharacter (Variables|Default|GetThirdPersonCharacter))
  ;[0.2915 1 0.5109] オーバーラップはじめ
  ;;[1 1 1] プライヤーかどうか
  (if (== OtherActor (Game|Player|GetPlayerPawn 0))
    ;;[1 1 1] プレイヤーを黄色とする
    (Variables|/Game/ThirdPersonBP/Blueprints/ThirdPersonCharacter.ThirdPersonCharacter_C|SetNowYellow _thirdpersoncharacter true)
    (Variables|/Game/ThirdPersonBP/Blueprints/ThirdPersonCharacter.ThirdPersonCharacter_C|SetNowRed _thirdpersoncharacter false)
    (Variables|/Game/ThirdPersonBP/Blueprints/ThirdPersonCharacter.ThirdPersonCharacter_C|SetNowGreen _thirdpersoncharacter false)
    (Variables|/Game/ThirdPersonBP/Blueprints/ThirdPersonCharacter.ThirdPersonCharacter_C|SetNowBlue _thirdpersoncharacter false)))

(event EventBeginPlay
  ;[1 0.8542 0.3886] 初期化
  (bind _outactors (Actor|GetAllActorsOfClass "/Game/ThirdPersonBP/Blueprints/ThirdPersonCharacter.ThirdPersonCharacter_C"))
  (for _array_element _outactors
    (Variables|Default|SetThirdPersonCharacter _array_element)))

(event Collision|EventActorBeginOverlap
  (params (OtherActor :type Actor%20Object%20Reference)))

(event EventTick
  (params (DeltaSeconds :type Float%20%28single-precision%29))
  (bind _returnvalue (Transformation|GetActorLocation))
  (bind _returnvalue_2 (Transformation|GetActorLocation))
  (bind _returnvalue_3 (Transformation|GetActorLocation))
  (bind _returnvalue_4 (Transformation|GetActorLocation))
  (bind _returnvalue_5 (+ (.x _returnvalue_3) -1.0))
  (bind _returnvalue_6 (+ (.x _returnvalue_4) 1.0))
  (bind _returnvalue_7 (+ (.y _returnvalue) 1.0))
  (bind _returnvalue_8 (+ (.y _returnvalue_2) -1.0))
  ;[1 0.496 0.6477] ループ
  (if (Variables|Default|GetMoveFlag)
    (if (Variables|Default|GetRIghtLeftFlag)
      (if (Variables|Default|GetOnPlusMove)
        (Transformation|SetActorLocation (Math|Vector|MakeVector (.x _returnvalue) _returnvalue_7 (.z _returnvalue)) false false)
        (if (>= _returnvalue_7 (Variables|Default|GetMaxValue))
          (Variables|Default|SetOnPlusMove false))
        (else
          (Transformation|SetActorLocation (Math|Vector|MakeVector (.x _returnvalue_2) _returnvalue_8 (.z _returnvalue_2)) false false)
          (if (>= (Variables|Default|GetLowValue) _returnvalue_8)
            (Variables|Default|SetOnPlusMove true))))
      (elif (Variables|Default|GetOnPlusMove)
        (Transformation|SetActorLocation (Math|Vector|MakeVector _returnvalue_6 (.y _returnvalue_4) (.z _returnvalue_4)) false false)
        (if (>= _returnvalue_6 (Variables|Default|GetMaxValue))
          (Variables|Default|SetOnPlusMove false))
        (else
          (Transformation|SetActorLocation (Math|Vector|MakeVector _returnvalue_5 (.y _returnvalue_3) (.z _returnvalue_3)) false false)
          (if (>= (Variables|Default|GetLowValue) _returnvalue_5)
            (Variables|Default|SetOnPlusMove true)))))))

(fn ConstructionScript)