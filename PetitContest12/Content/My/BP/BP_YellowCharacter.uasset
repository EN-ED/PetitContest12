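; BP_YellowCharacter is a yellow patrolling character that walks forward and halts when it sees the player in a non-yellow state.
; A detection box overlap sets PlayerWatch while the player is inside.
; Tick adds forward movement unless PlayerWatch is set and the cached ThirdPersonCharacter's NowYellow is false.
; Any capsule hit rotates the character 180 degrees, intended to turn it around at walls.
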(event OnComponentHit(CapsuleComponent)
  (params (HitComponent :type Primitive%20Component%20Object%20Reference) (OtherActor :type Actor%20Object%20Reference) (OtherComp :type Primitive%20Component%20Object%20Reference) (NormalImpulse :type Vector :default "0, 0, 0") (Hit :type Hit%20Result%20Structure%20%28by%20ref%29))
  ;[0.8807 1 0.4792] 壁に当たったら
  ;;[1 1 1] 回転させる
  (Transformation|SetActorRotation (Math|Rotator|CombineRotators (Transformation|GetActorRotation) "0,180.000000, 0")))

(event OnComponentBeginOverlap(PlayerWatchCollBox)
  (params (OverlappedComponent :type Primitive%20Component%20Object%20Reference) (OtherActor :type Actor%20Object%20Reference) (OtherComp :type Primitive%20Component%20Object%20Reference) (OtherBodyIndex :type Integer) (bFromSweep :type Boolean) (SweepResult :type Hit%20Result%20Structure%20%28by%20ref%29))
  ;[0.7186 1 0.7607] オーバーラップはじめ
  ;;[1 1 1] プレイヤーを見つけたら
  (if (== OtherActor (Game|Player|GetPlayerPawn 0))
    (Variables|Default|SetPlayerWatch true)))

(event OnComponentEndOverlap(PlayerWatchCollBox)
  (params (OverlappedComponent :type Primitive%20Component%20Object%20Reference) (OtherActor :type Actor%20Object%20Reference) (OtherComp :type Primitive%20Component%20Object%20Reference) (OtherBodyIndex :type Integer))
  ;[0.3304 0.9402 1] オーバーラップ終わり
  ;;[1 1 1] プレイヤーが見えなくなった
  (if (== OtherActor (Game|Player|GetPlayerPawn 0))
    (Variables|Default|SetPlayerWatch false)))

(event EventBeginPlay
  ;[1 1 1] 初期化
  (bind _outactors (Actor|GetAllActorsOfClass "/Game/ThirdPersonBP/Blueprints/ThirdPersonCharacter.ThirdPersonCharacter_C"))
  (for _array_element _outactors
    (Variables|Default|SetThirdPersonCharacter _array_element)))

(event Collision|EventActorBeginOverlap
  (params (OtherActor :type Actor%20Object%20Reference)))

(event EventTick
  (params (DeltaSeconds :type Float%20%28single-precision%29))
  ;[1 0.5751 0.6552] ループ
  ;;[1 1 1] プレイヤーを見つけたかどうか
  (if (Variables|Default|GetPlayerWatch)
    ;;[1 1 1] プレイヤーが黄色（ライトと同色）かどうか
    (if (Variables|/Game/ThirdPersonBP/Blueprints/ThirdPersonCharacter.ThirdPersonCharacter_C|GetNowYellow (Variables|Default|GetThirdPersonCharacter))
      ;;[1 1 1] 前に歩かせる
      (Pawn|Input|AddMovementInput (Transformation|GetActorForwardVector) (Variables|Default|GetSpeed) false :!label _label))
    (else
      (goto _label))))

(fn ConstructionScript)