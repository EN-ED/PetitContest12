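; Trigger-box actor that clears the player's color state and applies a blend body material while an overlap is active.
; On BeginPlay it caches the ThirdPersonCharacter found in the level.
; Box begin overlap resets its four NowBlue/Green/Red/Yellow flags and sets both mesh material slots to M_UE4Man_BodyBlend.
; End overlap restores the standard body and chest-logo materials; neither event checks which actor overlapped.
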(event OnComponentBeginOverlap(Box)
  (params (OverlappedComponent :type Primitive%20Component%20Object%20Reference) (OtherActor :type Actor%20Object%20Reference) (OtherComp :type Primitive%20Component%20Object%20Reference) (OtherBodyIndex :type Integer) (bFromSweep :type Boolean) (SweepResult :type Hit%20Result%20Structure%20%28by%20ref%29))
  (bind _thirdpersoncharacter (Variables|Default|GetThirdPersonCharacter))
  (bind _mesh (Variables|/Script/Engine.Character|GetMesh _thirdpersoncharacter))
  ;[0.6639 1 0.5915] オーバーラップはじめ
  ;;[1 1 1] 何色でもないとする
  (Variables|/Game/ThirdPersonBP/Blueprints/ThirdPersonCharacter.ThirdPersonCharacter_C|SetNowBlue _thirdpersoncharacter false)
  (Variables|/Game/ThirdPersonBP/Blueprints/ThirdPersonCharacter.ThirdPersonCharacter_C|SetNowGreen _thirdpersoncharacter false)
  (Variables|/Game/ThirdPersonBP/Blueprints/ThirdPersonCharacter.ThirdPersonCharacter_C|SetNowRed _thirdpersoncharacter false)
  (Variables|/Game/ThirdPersonBP/Blueprints/ThirdPersonCharacter.ThirdPersonCharacter_C|SetNowYellow _thirdpersoncharacter false)
  ;;[1 1 1] マテリアルを透過通常色のモノにする
  (Rendering|Material|SetMaterial _mesh 0 "/Game/My/Material/M_UE4Man_BodyBlend.M_UE4Man_BodyBlend")
  (Rendering|Material|SetMaterial _mesh 1 "/Game/My/Material/M_UE4Man_BodyBlend.M_UE4Man_BodyBlend"))

(event OnComponentEndOverlap(Box)
  (params (OverlappedComponent :type Primitive%20Component%20Object%20Reference) (OtherActor :type Actor%20Object%20Reference) (OtherComp :type Primitive%20Component%20Object%20Reference) (OtherBodyIndex :type Integer))
  (bind _thirdpersoncharacter (Variables|Default|GetThirdPersonCharacter))
  (bind _mesh (Variables|/Script/Engine.Character|GetMesh _thirdpersoncharacter))
  ;[1 0.7464 0.2956] オーバーラップ終わり
  ;;[1 1 1] マテリアルを通常のモノにする
  (Rendering|Material|SetMaterial _mesh 0 "/Game/Mannequin/Character/Materials/M_UE4Man_Body.M_UE4Man_Body")
  (Rendering|Material|SetMaterial _mesh 1 "/Game/Mannequin/Character/Materials/M_UE4Man_ChestLogo.M_UE4Man_ChestLogo"))

(event EventBeginPlay
  ;[0.9059 0.4464 1] 初期化
  ;;[1 1 1] プレイヤークラスを変数化
  (bind _outactors (Actor|GetAllActorsOfClass "/Game/ThirdPersonBP/Blueprints/ThirdPersonCharacter.ThirdPersonCharacter_C"))
  (for _array_element _outactors
    (Variables|Default|SetThirdPersonCharacter _array_element)))

(event Collision|EventActorBeginOverlap
  (params (OtherActor :type Actor%20Object%20Reference)))

(event EventTick
  (params (DeltaSeconds :type Float%20%28single-precision%29)))

(fn ConstructionScript)