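; BP_GreenCharacter is a patrolling character that reacts to the player's color.
; It walks forward slowly on Tick and turns around whenever its capsule hits something.
; A PlayerWatchCollBox overlap flags the player as seen, which halts walking unless the player's NowGreen is set (matching the light color, per the comments).
; BeginPlay caches the ThirdPersonCharacter reference used for that color check.
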(event OnComponentHit(CapsuleComponent)
  (params (HitComponent :type Primitive%20Component%20Object%20Reference) (OtherActor :type Actor%20Object%20Reference) (OtherComp :type Primitive%20Component%20Object%20Reference) (NormalImpulse :type Vector :default "0, 0, 0") (Hit :type Hit%20Result%20Structure%20%28by%20ref%29))
  ;[1 1 1] 回転させる
  (Transformation|SetActorRotation (Math|Rotator|CombineRotators (Transformation|GetActorRotation) "0,180.000000, 0")))

(event OnComponentBeginOverlap(PlayerWatchCollBox)
  (params (OverlappedComponent :type Primitive%20Component%20Object%20Reference) (OtherActor :type Actor%20Object%20Reference) (OtherComp :type Primitive%20Component%20Object%20Reference) (OtherBodyIndex :type Integer) (bFromSweep :type Boolean) (SweepResult :type Hit%20Result%20Structure%20%28by%20ref%29))
  ;[1 1 1] 位置的にプレイヤーを見つけたら見つけたとする
  (if (== OtherActor (Game|Player|GetPlayerPawn 0))
    (Variables|Default|SetPlayerWatch true)))

(event OnComponentEndOverlap(PlayerWatchCollBox)
  (params (OverlappedComponent :type Primitive%20Component%20Object%20Reference) (OtherActor :type Actor%20Object%20Reference) (OtherComp :type Primitive%20Component%20Object%20Reference) (OtherBodyIndex :type Integer))
  ;[1 1 1] 位置的にプレイヤーが離れたら
  (if (== OtherActor (Game|Player|GetPlayerPawn 0))
    (Variables|Default|SetPlayerWatch false)))

(event EventBeginPlay
  (bind _outactors (Actor|GetAllActorsOfClass "/Game/ThirdPersonBP/Blueprints/ThirdPersonCharacter.ThirdPersonCharacter_C"))
  (for _array_element _outactors
    (Variables|Default|SetThirdPersonCharacter _array_element)))

(event Collision|EventActorBeginOverlap
  (params (OtherActor :type Actor%20Object%20Reference)))

(event EventTick
  (params (DeltaSeconds :type Float%20%28single-precision%29))
  ;[1 1 1] プレイヤーを見つけたかどうか
  (if (Variables|Default|GetPlayerWatch)
    ;[1 1 1] プレイヤーが緑色（ライトと同色）かどうか
    (if (Variables|/Game/ThirdPersonBP/Blueprints/ThirdPersonCharacter.ThirdPersonCharacter_C|GetNowGreen (Variables|Default|GetThirdPersonCharacter))
      ;[1 1 1] 前に歩かせる
      (Pawn|Input|AddMovementInput (Transformation|GetActorForwardVector) 0.3 false :!label _label))
    (else
      (goto _label))))

(fn ConstructionScript)