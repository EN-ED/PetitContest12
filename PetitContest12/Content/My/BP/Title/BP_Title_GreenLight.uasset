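; BP_Title_GreenLight is a title-screen actor that slides past the character and turns it green.
; BeginPlay caches the ThirdPersonCharacter, and Tick moves the actor along negative X until a flag stops it once off-screen.
; Passing the character's X position, or the Cube overlapping the player pawn, applies the green material to the mesh and sets the character's NowGreen flag.
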(event OnComponentBeginOverlap(Cube)
  (params (OverlappedComponent :type Primitive%20Component%20Object%20Reference) (OtherActor :type Actor%20Object%20Reference) (OtherComp :type Primitive%20Component%20Object%20Reference) (OtherBodyIndex :type Integer) (bFromSweep :type Boolean) (SweepResult :type Hit%20Result%20Structure%20%28by%20ref%29))
  (bind _thirdpersoncharacter (Variables|Default|GetThirdPersonCharacter))
  (bind _mesh (Variables|/Script/Engine.Character|GetMesh _thirdpersoncharacter))
  (if (== OtherActor (Game|Player|GetPlayerPawn 0))
    (Rendering|Material|SetMaterial _mesh 0 "/Game/My/Material/M_Green.M_Green")
    (Rendering|Material|SetMaterial _mesh 1 "/Game/My/Material/M_Green.M_Green")
    (Variables|/Game/ThirdPersonBP/Blueprints/ThirdPersonCharacter.ThirdPersonCharacter_C|SetNowGreen _thirdpersoncharacter true)))

(event EventBeginPlay
  ;[1 0.005931 0] 初期化
  ;;[1 1 1] キャラクタークラスを変数化（一体だけなのでGet All Actors Of Class使用）
  (bind _outactors (Actor|GetAllActorsOfClass "/Game/ThirdPersonBP/Blueprints/ThirdPersonCharacter.ThirdPersonCharacter_C"))
  (for _array_element _outactors
    (Variables|Default|SetThirdPersonCharacter _array_element)))

(event Collision|EventActorBeginOverlap
  (params (OtherActor :type Actor%20Object%20Reference)))

(event EventTick
  (params (DeltaSeconds :type Float%20%28single-precision%29))
  (bind _returnvalue (Transformation|GetActorLocation))
  (bind _thirdpersoncharacter (Variables|Default|GetThirdPersonCharacter))
  (bind _mesh (Variables|/Script/Engine.Character|GetMesh _thirdpersoncharacter))
  ;[0 1 0.2441] ループ
  ;;[1 1 1] キャラクターのいる位置に着いたら
  (if (<= (.x (Transformation|GetActorLocation)) -1.46e+03)
    ;;[1 1 1] キャラクターのマテリアルの色を緑に変える
    (Rendering|Material|SetMaterial _mesh 0 "/Game/My/Material/M_Green.M_Green")
    (Rendering|Material|SetMaterial _mesh 1 "/Game/My/Material/M_Green.M_Green")
    (Variables|/Game/ThirdPersonBP/Blueprints/ThirdPersonCharacter.ThirdPersonCharacter_C|SetNowGreen _thirdpersoncharacter true))
  (if (not (Variables|Default|GetOnPlusMove))
    ;;[1 1 1] 動かす
    (Transformation|SetActorLocation (Math|Vector|MakeVector (+ (.x _returnvalue) -5.0) 0.0 0.0) false false)
    ;;[1 1 1] 画面外に行ったら動かせないようにする
    (if (<= (.x _returnvalue) -4e+03)
      (Variables|Default|SetOnPlusMove true))))

(fn ConstructionScript)