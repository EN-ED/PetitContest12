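; Title-screen green character that walks forward endlessly, teleporting back to its start once it moves off screen.
; BeginPlay caches the ThirdPersonCharacter, and Tick changes that character's mesh materials based on this actor's X position.
; Inside the light-overlap band it applies a translucent green blend; outside it applies solid green if NowGreen is set.
; Hit and player-detection handlers are empty, with their former logic left disconnected.
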(event OnComponentHit(CapsuleComponent)
  (params (HitComponent :type Primitive%20Component%20Object%20Reference) (OtherActor :type Actor%20Object%20Reference) (OtherComp :type Primitive%20Component%20Object%20Reference) (NormalImpulse :type Vector :default "0, 0, 0") (Hit :type Hit%20Result%20Structure%20%28by%20ref%29))
  ;[1 1 1] 使ってない処理
)

(event OnComponentBeginOverlap(PlayerWatchCollBox)
  (params (OverlappedComponent :type Primitive%20Component%20Object%20Reference) (OtherActor :type Actor%20Object%20Reference) (OtherComp :type Primitive%20Component%20Object%20Reference) (OtherBodyIndex :type Integer) (bFromSweep :type Boolean) (SweepResult :type Hit%20Result%20Structure%20%28by%20ref%29))
  ;[1 1 1] 使ってない処理
)

(event OnComponentEndOverlap(PlayerWatchCollBox)
  (params (OverlappedComponent :type Primitive%20Component%20Object%20Reference) (OtherActor :type Actor%20Object%20Reference) (OtherComp :type Primitive%20Component%20Object%20Reference) (OtherBodyIndex :type Integer))
  ;[1 1 1] 使ってない処理
)

(event EventBeginPlay
  ;[1 0 0.06395] 初期化
  ;;[1 1 1] キャラクタークラスを変数化
  (bind _outactors (Actor|GetAllActorsOfClass "/Game/ThirdPersonBP/Blueprints/ThirdPersonCharacter.ThirdPersonCharacter_C"))
  (for _array_element _outactors
    (Variables|Default|SetThirdPersonCharacter _array_element)))

(event Collision|EventActorBeginOverlap
  (params (OtherActor :type Actor%20Object%20Reference)))

(event EventTick
  (params (DeltaSeconds :type Float%20%28single-precision%29))
  (bind _returnvalue (Transformation|GetActorLocation))
  (bind _thirdpersoncharacter (Variables|Default|GetThirdPersonCharacter))
  (bind _thirdpersoncharacter_2 (Variables|Default|GetThirdPersonCharacter))
  (bind _mesh (Variables|/Script/Engine.Character|GetMesh _thirdpersoncharacter))
  (bind _mesh_2 (Variables|/Script/Engine.Character|GetMesh _thirdpersoncharacter_2))
  ;[0 1 0.05136] ループ
  ;;[1 1 1] 前に歩かせる
  (Pawn|Input|AddMovementInput (Transformation|GetActorForwardVector) 1e+01 false)
  ;;[1 1 1] キャラクターにライトが重なるタイミング
  (if (<= (.x _returnvalue) -6.9e+02)
    ;;[1 1 1] キャラクターにライトが重ならないライン
    (if (>= (.x _returnvalue) -1.64e+03)
      ;;[1 1 1] キャラクターのマテリアルを緑透過色に変える
      (Rendering|Material|SetMaterial _mesh_2 0 "/Game/My/Material/M_UE4Man_BodyGreenBlend.M_UE4Man_BodyGreenBlend")
      (Rendering|Material|SetMaterial _mesh_2 1 "/Game/My/Material/M_UE4Man_BodyGreenBlend.M_UE4Man_BodyGreenBlend")
      (else
        ;;[1 1 1] キャラクターが緑ライトを通過した後の状態だったらマテリアルを緑色に変える
        (if (Variables|/Game/ThirdPersonBP/Blueprints/ThirdPersonCharacter.ThirdPersonCharacter_C|GetNowGreen _thirdpersoncharacter) :!label _label
          (Rendering|Material|SetMaterial _mesh 0 "/Game/My/Material/M_Green.M_Green")
          (Rendering|Material|SetMaterial _mesh 1 "/Game/My/Material/M_Green.M_Green"))))
    (else
      (goto _label)))
  ;;[1 1 1] 画面外に行ったら元の位置に戻させる
  (if (<= (.x (Transformation|GetActorLocation)) -2.2e+03)
    (Transformation|SetActorLocation (Math|Vector|MakeVector 2.4e+03 1e+01 226.001602) false true)))

(fn ConstructionScript)